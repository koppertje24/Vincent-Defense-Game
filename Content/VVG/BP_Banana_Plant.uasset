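; Buildable banana plant placeable that works as a crafting station, apparently adapted from a campfire, whose name it still shows on interaction.
; Supplies a floor checker and build collision for placement; once built, the server initializes its container and links it to the crafting component.
; Releasing interact opens the crafting UI in queue-only mode.
; Replicated TurnedOn state has an empty update, and its toggle, default loot and waste logic are disconnected.
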(event EventTryInteractBPI
  (params (Release :type Boolean) (PlayerController :type Player%20Controller%20Object%20Reference))
  ;[1 1 1] Interactions.
  (if Release
    (Class|BPIPlayer|OpenCraftingPlaceBPI(Message) PlayerController (Variables|Default|GetCraftingComponent) (Variables|Default|GetContainerComponent) true)))

(event EventBeginPlay
  (bind _containercomponent (Variables|Default|GetContainerComponent))
  ;[1 1 1] Begin play.
  (|CallParentFunction)
  (if (Variables|Default|GetBuilt)
    (Networking|SwitchHasAuthority
      (:Authority
        (Default|InitComponent _containercomponent)
        (Default|InitComponent (Variables|Default|GetCraftingComponent) _containercomponent)))))

(event EventSetFloorCheckers
  ;[1 1 1] Overridden Events.
  (Variables|Default|SetFloorCheckers (Utilities|Array|MakeArray (Variables|Default|GetFloorChecker1))))

(event EventDestroyBuildComponents
  ;[1 1 1] Overridden Events.
  (Components|DestroyComponent (Variables|Default|GetBuildCollision)))

(fn ConstructionScript
  (|CallParentFunction))

(fn CheckBuildCollisions
  (params (Actor :type Actor%20Object%20Reference))
  (return (CallFunction|CheckActorCollisions Actor (Variables|Default|GetBuildCollision))))

(fn OnRepTurnedon
  (Campfire|UpdateTurnedon))

(fn UpdateTurnedon)

(fn CheckCanInteractBPI
  (params (PlayerController :type Player%20Controller%20Object%20Reference))
  (return true))

(fn GetInteractionObjectNameBPI
  (return "Campfire"))

(fn GetInteractionTextBPI
  (params (PlayerController :type Player%20Controller%20Object%20Reference))
  (return "Campfire"))

(fn IsTurnedonBPI
  (return (Variables|Campfire|GetTurnedOn)))