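; Quest task component that completes when no character with a given tag is left alive.
; On init and whenever the player kills a character, it recounts tagged BP_Character_Base actors with health above zero and broadcasts a progress update.
; A zero count on a kill or load check marks the task finished.
; The count feeds the progress text, and loading re-evaluates the world instead of using the saved value.
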(event Custom|CheckProgress
  (params (Character :type BP%20Character%20Base%20Object%20Reference))
  (CallFunction|UpdateAliveEnemy's)
  (if (> (Variables|Default|GetAlive%20enemy's) 0)
    (Variables|Default|Setno%20enemy's%20Left false)
    (else
      (Variables|Default|Setno%20enemy's%20Left true)
      (Variables|Default|SetIsFinished true)
      (CallFunction|CheckFinished))))

(event EventInitComponent
  (params (PlayerManagerComponent :type BP%20Player%20Manager%20Component%20Object%20Reference))
  (|CallParentFunction PlayerManagerComponent)
  (EventDispatchers|BindEventtoOnPlayerKillCharacter PlayerManagerComponent (delegate Custom|CheckProgress))
  (CallFunction|UpdateAliveEnemy's))

(fn GetProgress
  (return (Utilities|String|ToString(Integer) (Variables|Default|GetAlive%20enemy's))))

(fn GetProgressText
  (return (Utilities|Text|FormatText (Variables|Default|GetProgressTextFormat) (Variables|Default|GetAlive%20enemy's))))

(fn LoadProgress
  (params (Progress :type String))
  (CallFunction|CheckProgress)
  (return true))

(fn UpdateAliveEnemy's
  (Variables|Default|SetAlive%20enemy's 0)
  (bind _outactors (Actor|GetAllActorswithTag (Variables|Default|GetTag)))
  (for _array_element _outactors
    (bind _asbp_character_base (Utilities|Casting|CastToBP_Character_Base _array_element))
    (bind _health (Default|GetHealthInfoBPI _asbp_character_base))
    (if (> _health 0.0)
      (Variables|Default|SetAlive%20enemy's (+ (Variables|Default|GetAlive%20enemy's) 1))))
  (Default|CallOnProgressUpdated self)
  (return))