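; Garden building piece that players can always interact with, labeled "Bed", carrying an owner list, owned flag and ownership distance.
; It supplies four floor checkers and a build collision to the parent's placement logic, destroying the collision with the build components.
; Interaction prompts Authorize or Deauthorize by player name, but the handler only opens or closes the HUD mallet menu.
; Save and load overrides persist ownership data by SaveID after the parent call succeeds.
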(event EventTryInteractBPI
  (params (Release :type Boolean) (PlayerController :type Player%20Controller%20Object%20Reference))
  (bind _returnvalue (HUD|GetHUD PlayerController))
  ;[1 1 1] Interactions.
  (if Release
    (Class|BPIHUDGame|OpenMalletMenuBPI(Message) _returnvalue)
    (else
      (Class|BPIHUDGame|CloseMalletMenuBPI(Message) _returnvalue))))

(event EventSetFloorCheckers
  ;[1 1 1] Overridden Events.
  (Variables|Default|SetFloorCheckers (Utilities|Array|MakeArray (Variables|Default|GetFloorChecker1) (Variables|Default|GetFloorChecker2) (Variables|Default|GetFloorChecker3) (Variables|Default|GetFloorChecker4))))

(event EventDestroyBuildComponents
  ;[1 1 1] Overridden Events.
  (Components|DestroyComponent (Variables|Default|GetBuildCollision)))

(fn ConstructionScript
  (|CallParentFunction))

(fn CheckBuildCollisions
  (params (Actor :type Actor%20Object%20Reference))
  (return (CallFunction|CheckActorCollisions Actor (Variables|Default|GetBuildCollision))))

(fn SaveDataBPI
  (params (SaveData :type Save%20Game%20Object%20Reference))
  (bind _success (|CallParentFunction SaveData))
  (if _success
    (bind _success_2 (Class|BPIGameSave|SetOwnershipSaveDataBPI(Message) SaveData (Variables|Default|GetSaveID) (Utilities|Struct|MakeSTR_SaveData_Ownership (Variables|Totem|GetIsOwned) (Variables|Totem|GetOwnerNames) (Variables|Totem|GetOwnershipDistance))))
    (return _success_2)
    (else
      (return false))))

(fn LoadDataBPI
  (params (SaveData :type Save%20Game%20Object%20Reference))
  (bind _success (|CallParentFunction SaveData))
  (if _success
    (bind (_success_2 _ownershipsavedata) (Class|BPIGameSave|GetOwnershipSaveDataBPI(Message) SaveData (Variables|Default|GetSaveID)))
    (if _success_2
      (Variables|Totem|SetIsOwned (.IsOwned (Utilities|Struct|BreakSTR_SaveData_Ownership _ownershipsavedata)))
      (Variables|Totem|SetOwnerNames (.PlayerNames (Utilities|Struct|BreakSTR_SaveData_Ownership _ownershipsavedata)))
      (Variables|Totem|SetOwnershipDistance (.OwnershipDistance (Utilities|Struct|BreakSTR_SaveData_Ownership _ownershipsavedata)))
      (return true)
      (else
        _)))
  (return false))

(fn CheckCanInteractBPI
  (params (PlayerController :type Player%20Controller%20Object%20Reference))
  (return true))

(fn CheckPlayerIsOwnerBPI
  (params (PlayerController :type Player%20Controller%20Object%20Reference))
  (return (Utilities|Array|ContainsItem (Variables|Totem|GetOwnerNames) (PlayerState|GetPlayerName (Variables|/Script/Engine.Controller|GetPlayerState PlayerController)))))

(fn GetInteractionObjectNameBPI
  (return "Bed"))

(fn GetInteractionTextBPI
  (params (PlayerController :type Player%20Controller%20Object%20Reference))
  (bind _isowner (CallFunction|CheckPlayerIsOwnerBPI PlayerController))
  (return (select _isowner "Deauthorize" "Authorize")))

(fn GetOwnersBPI
  (return (Variables|Totem|GetOwnerNames)))

(fn GetOwnershipInfoBPI
  (return (Variables|Totem|GetIsOwned) (Variables|Totem|GetOwnerNames) (Variables|Totem|GetOwnershipDistance)))

(fn IsTurnedonBPI
  (return false))