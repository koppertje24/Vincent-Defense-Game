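; Buildable well that produces buckets of water through a loading-bar interaction.
; Releasing interact opens the HUD loading-bar menu, and each call to its fill function advances progress by a tick.
; A full bar spawns a Bucket_of_water item from the items data table at SpawnLocation, then resets on the next call.
; Build-placement hooks use BuildCollision and FloorChecker1; the TurnedOn update is empty, and the object name returns "Campfire".
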(event EventTryInteractBPI
  (params (Release :type Boolean) (PlayerController :type Player%20Controller%20Object%20Reference))
  ;[1 1 1] Interactions.
  (if Release
    (Class|BPIHUDGame|OpenLoadingbarMenuBPI(Message) (HUD|GetHUD PlayerController) self)))

(event EventBeginPlay
  ;[1 1 1] Begin play.
  (|CallParentFunction)
  (if (Variables|Default|GetBuilt)
    _))

(event EventSetFloorCheckers
  ;[1 1 1] Overridden Events.
  (Variables|Default|SetFloorCheckers (Utilities|Array|MakeArray (Variables|Default|GetFloorChecker1))))

(event EventDestroyBuildComponents
  ;[1 1 1] Overridden Events.
  (Components|DestroyComponent (Variables|Default|GetBuildCollision)))

(fn ConstructionScript
  (|CallParentFunction))

(fn CheckBuildCollisions
  (params (Actor :type Actor%20Object%20Reference))
  (return (CallFunction|CheckActorCollisions Actor (Variables|Default|GetBuildCollision))))

(fn OnRepTurnedon
  (Campfire|UpdateTurnedon))

(fn UpdateTurnedon)

(fn LoadbarMenuFill
  (return (/ (Variables|Default|GetCurrentLoadbarFill) (Variables|Default|GetMaxLoadbarFill))))

(fn LoadbarMenuFunction
  (bind _loadbar_fill (CallFunction|LoadbarMenuFill))
  (if (>= _loadbar_fill 1.0)
    (bind _output_get (Variables|Default|SetCurrentLoadbarFill 0.0))
    (return _output_get)
    (else
      (Variables|Default|SetCurrentLoadbarFill (+ (Variables|Default|GetCurrentLoadbarFill) (Variables|Default|GetTickLoadbarFill)))
      (bind _loadbar_fill_2 (CallFunction|LoadbarMenuFill))
      (if (>= _loadbar_fill_2 1.0)
        (bind _returnvalue (Utilities|GetDataTableRow "/Game/VVG/DataTable/DT_Items_VVG.DT_Items_VVG" "Bucket_of_water")
          (:then
            (Class|BPIGameInstance|SpawnItemsBPI(Message) (Game|GetGameInstance) (Utilities|Array|MakeArray (Utilities|Struct|MakeSTR_Item (.itemhandle _returnvalue) 1 -1 -1.0 -1.0)) (Transformation|GetWorldLocation (Variables|Default|GetSpawnLocation)) 0.0 0.0 1.0 1.0)
            (return _loadbar_fill_2)))
        (else
          (return _loadbar_fill_2))))))

(fn CheckCanInteractBPI
  (params (PlayerController :type Player%20Controller%20Object%20Reference))
  (return true))

(fn GetInteractionObjectNameBPI
  (return "Campfire"))

(fn GetInteractionTextBPI
  (params (PlayerController :type Player%20Controller%20Object%20Reference))
  (return "Well"))

(fn IsTurnedonBPI
  (return (Variables|Campfire|GetTurnedOn)))