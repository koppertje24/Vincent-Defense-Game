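; Base building object in EasySurvivalRPG for pieces placed on floors or landscape, handling their snapping and placement validation.
; Child classes supply floor checkers through SetFloorCheckers, and CheckSupport requires each to overlap an allowed surface, chosen by the PlacedOnLandscape and PlacedOnFloor flags.
; CheckBuildStatus allows building only with support and when all overlapping actors pass CheckBuildCollisions.
; GetSnapPosition takes height from the target floor, optionally rounds XY to a grid, and adds a yaw-rotated offset.
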(fn ConstructionScript
  (|CallParentFunction)
  (CallFunction|SetFloorCheckers))

(fn CheckSupport
  (bind _placedonlandscape (Variables|Default|GetPlacedOnLandscape))
  (LocalVariables|SetLocalFloorCheck true)
  (for _array_element (Variables|State|GetFloorCheckers)
    (if (and _placedonlandscape (Variables|Consts|GetPlacedOnFloor))
      (if (and (not (CallFunction|HasLandscape (Collision|GetOverlappingActors _array_element 0 :!class /Script/Engine.PrimitiveComponent))) (not (CallFunction|HasFloor (Collision|GetOverlappingActors _array_element "/Game/VVG/BP_Building_BuildingObject.BP_Building_BuildingObject_C" :!class /Script/Engine.PrimitiveComponent))))
        (LocalVariables|SetLocalFloorCheck false :!label _label)
        (return (LocalVariables|GetLocalFloorCheck)))
      (elif _placedonlandscape
        (if (not (CallFunction|HasLandscape (Collision|GetOverlappingActors _array_element 0 :!class /Script/Engine.PrimitiveComponent)))
          (goto _label))
        (elif (not (CallFunction|HasFloor (Collision|GetOverlappingActors _array_element "/Game/VVG/BP_Building_BuildingObject.BP_Building_BuildingObject_C" :!class /Script/Engine.PrimitiveComponent)))
          (goto _label)))))
  (return (LocalVariables|GetLocalFloorCheck)))

(fn CheckBuildStatus
  (params (TargetObject :type BP%20Building%20Building%20Object%20Object%20Reference))
  (bind _self self)
  (bind _overlappingactors (Collision|GetOverlappingActors _self 0 :!class /Script/Engine.Actor))
  ;[1 1 1] Check Floor Object can be build.
  (bind _result (CallFunction|CheckSupport))
  (if _result
    (LocalVariables|SetLocalCount (Utilities|Array|Length _overlappingactors))
    (for _array_element _overlappingactors
      (if (CallFunction|CheckBuildCollisions _array_element)
        (Math|Integer|DecrementInt (LocalVariables|GetLocalCount))))
    (if (== (LocalVariables|GetLocalCount) 0)
      (return true)
      (else
        _)))
  (return false))

(fn CheckSnap
  (params (TargetObject :type BP%20Building%20Building%20Object%20Object%20Reference))
  (return (Variables|/Game/VVG/BP_Building_BuildingObject.BP_Building_BuildingObject_C|GetIsFloor TargetObject)))

(fn GetSnapPosition
  (params (TargetObject :type BP%20Building%20Building%20Object%20Object%20Reference) (InputRotation :type Float%20%28single-precision%29) (HitLocation :type Vector :default "0, 0, 0") (GridMode :type Boolean) (SnappingMode :type Boolean))
  (bind (_x _y) (Math|Vector|BreakVector HitLocation))
  (bind _returnvalue (Math|Rotator|MakeRotator 0.0 0.0 InputRotation))
  (bind (_gridoffset _gridpropsoffset _gridcorrectoffset) (Utilities|GetGridOffset GridMode))
  ;[1 1 1] Get snap location and rotation of Floor Object and Target Unit.
  (if (Variables|/Game/VVG/BP_Building_BuildingObject.BP_Building_BuildingObject_C|GetIsFloor TargetObject)
    (LocalVariables|SetLocalZ (Default|GetFloorZ TargetObject))
    (return (+ (Math|Vector|MakeVector (select GridMode (+ (* (Math|Float|Round (/ (- _x _gridcorrectoffset) _gridpropsoffset)) _gridpropsoffset) _gridcorrectoffset) _x) (select GridMode (+ (* (Math|Float|Round (/ (- _y _gridcorrectoffset) _gridpropsoffset)) _gridpropsoffset) _gridcorrectoffset) _y) (LocalVariables|GetLocalZ)) (Math|Vector|RotateVector _gridoffset _returnvalue)) _returnvalue)))

(fn SetFloorCheckers
  ;[1 1 1] Sets an array for floor checking. Overridden in child class.
)

(fn HasFloor
  (params (Actors :type Array%20of%20Actor%20Object%20References))
  ;[1 1 1] Returns true if actors array contains floor.
  (for _array_element Actors
    (bind _asbp_building_building_object (Utilities|Casting|CastToBP_Building_BuildingObject _array_element))
    (if (and (Variables|/Game/VVG/BP_Building_BuildingObject.BP_Building_BuildingObject_C|GetIsFloor _asbp_building_building_object) (!= _asbp_building_building_object self))
      (return true)))
  (return false))