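; Base building object for wall-mounted props in the survival RPG's building system, validating and orienting placement against walls.
; Placement requires every prop checker to overlap a wall or right triangle wall, and all overlapping actors to pass the build-collision check.
; Snapping accepts four building types, keeps the hit location and flips yaw 180 degrees according to the side hit.
; Child classes can override SetWallCheckers to supply their own support checkers.
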(event EventDestroyBuildComponents
  ;[1 1 1] Overridden events.
  (Components|DestroyComponent (Variables|Default|GetBuildCollision)))

(fn ConstructionScript
  (|CallParentFunction)
  (CallFunction|SetWallCheckers))

(fn CheckSupport
  (LocalVariables|SetLocalWallCheck true)
  (for _array_element (Variables|Default|GetPropCheckers)
    (if (not (CallFunction|HasWall (Collision|GetOverlappingActors _array_element 0 :!class /Script/Engine.PrimitiveComponent)))
      (LocalVariables|SetLocalWallCheck false)
      (return (LocalVariables|GetLocalWallCheck))))
  (return (LocalVariables|GetLocalWallCheck)))

(fn CheckSnap
  (params (TargetObject :type BP%20Building%20Building%20Object%20Object%20Reference))
  (bind _buildingtype (Variables|/Game/VVG/BP_Building_BuildingObject.BP_Building_BuildingObject_C|GetBuildingType TargetObject))
  (return (Math|Boolean|ORBoolean (Utilities|Enum|Equal(Enum) _buildingtype "NewEnumerator3") (Utilities|Enum|Equal(Enum) _buildingtype "NewEnumerator4") (Utilities|Enum|Equal(Enum) _buildingtype "NewEnumerator5") (Utilities|Enum|Equal(Enum) _buildingtype "NewEnumerator17"))))

(fn CheckBuildCollisions
  (params (Actor :type Actor%20Object%20Reference))
  (return (CallFunction|CheckActorCollisions Actor (Variables|Default|GetBuildCollision))))

(fn CheckBuildStatus
  (params (TargetObject :type BP%20Building%20Building%20Object%20Object%20Reference))
  (bind _self self)
  (bind _overlappingactors (Collision|GetOverlappingActors _self 0 :!class /Script/Engine.Actor))
  (bind _result (CallFunction|CheckSupport))
  (if _result
    (LocalVariables|SetLocalCount (Utilities|Array|Length _overlappingactors))
    (for _array_element _overlappingactors
      (if (CallFunction|CheckBuildCollisions _array_element)
        (Math|Integer|DecrementInt (LocalVariables|GetLocalCount))))
    (if (== (LocalVariables|GetLocalCount) 0)
      (return true)
      (else
        _)))
  (return false))

(fn GetSnapPosition
  (params (TargetObject :type BP%20Building%20Building%20Object%20Object%20Reference) (InputRotation :type Float%20%28single-precision%29) (HitLocation :type Vector :default "0, 0, 0") (GridMode :type Boolean) (SnappingMode :type Boolean))
  (bind _returnvalue (Transformation|GetActorRotation TargetObject))
  (bind _returnvalue_2 (Transformation|GetActorLocation TargetObject))
  (bind _returnvalue_3 (- HitLocation _returnvalue_2))
  (bind _yaw (Math|Rotator|BreakRotator _returnvalue))
  (bind (_x _y) (Math|Vector|BreakVector _returnvalue_3))
  (return HitLocation (select (> (- (* _y (Math|Trig|Cos(Degrees) _yaw)) (* _x (Math|Trig|Sin(Degrees) _yaw))) 0.0) _returnvalue (Math|Rotator|CombineRotators _returnvalue "0,180.000000, 0"))))

(fn HasWall
  (params (Actors :type Array%20of%20Actor%20Object%20References))
  ;[1 1 1] Returns true if array of actors has wall.
  (for _array_element Actors
    (Utilities|Casting|CastToBP_Building_Wall _array_element
      (:then
        _)
      (:CastFailed
        (Utilities|Casting|CastToBP_Building_TriangleWall_Right _array_element)))
    (return true))
  (return false))

(fn SetWallCheckers
  (bind _propcheckers (Variables|Default|GetPropCheckers))
  ;[1 1 1] Sets an array for wall checking. Overridden in child class.
  (Utilities|Array|Clear _propcheckers)
  (Utilities|Array|Add _propcheckers (Variables|Default|GetCheckPropCollision)))