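; Modular building door frame for the survival RPG that swings and manages its attached door.
; Multicast open and close events play or reverse a timeline that rotates DoorAxis in yaw.
; A dot product picks swing direction from player 0's side of the frame, evaluated per machine, so clients can differ.
; Removing attached objects cascades into and destroys the door, optionally multicasting its destructible mesh.
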(event Custom|OpenDoor%20%28Multicast%29
  (bind _defaultsceneroot (Variables|Default|GetDefaultSceneRoot))
  ;[1 1 1] Open and Close door.
  (Utilities|IsValid (Variables|References|GetDoorReference)
    (:Is%20Valid
      ;[1 1 1] personal touch
      (if (< (Math|Vector|DotProduct (Math|Vector|Normalize (- (Transformation|GetWorldLocation _defaultsceneroot) (Transformation|GetActorLocation (Game|GetPlayerCharacter 0)))) (Math|Vector|GetRightVector _defaultsceneroot)) 0.0)
        (Variables|Default|SetOpendoorMultiplier -1.0)
        (bind _rotationz (Timeline|OpenDoorTimeline Play)
          (:Update
            (Transformation|SetRelativeRotation (Variables|Default|GetDoorAxis) (Math|Rotator|MakeRotator 0.0 0.0 (* _rotationz (Variables|Default|GetOpendoorMultiplier))) false true)))
        (else
          (Variables|Default|SetOpendoorMultiplier 1.0)
          (Timeline|OpenDoorTimeline Play))))))

(event Custom|CloseDoor%20%28Multicast%29
  ;[1 1 1] Open and Close door.
  (Utilities|IsValid (Variables|References|GetDoorReference)
    (:Is%20Valid
      (bind _rotationz (Timeline|OpenDoorTimeline Reverse)
        (:Update
          (Transformation|SetRelativeRotation (Variables|Default|GetDoorAxis) (Math|Rotator|MakeRotator 0.0 0.0 (* _rotationz (Variables|Default|GetOpendoorMultiplier))) false true))))))

(event EventRemoveAttachedObject
  (params (Destruct :type Boolean))
  (bind _doorreference (Variables|References|GetDoorReference))
  ;[1 1 1] Overrided Events.
  (Utilities|IsValid _doorreference
    (:Is%20Valid
      (if Destruct
        (CallFunction|Destruct(Multicast) (.DestructibleMesh (Utilities|Struct|BreakSTR_BuildingObjectSettings (Variables|/Game/EasySurvivalRPG/Blueprints/InteractionObjects/BuildingObjects/Base/BP_Building_BuildingObject.BP_Building_BuildingObject_C|GetSettings _doorreference))) (Transformation|GetWorldTransform (Variables|/Game/EasySurvivalRPG/Blueprints/InteractionObjects/BuildingObjects/Base/BP_Building_BuildingObject.BP_Building_BuildingObject_C|GetMesh _doorreference))))
      (Default|RemoveAttachedObject _doorreference Destruct)
      (Actor|DestroyActor _doorreference))))

(fn ConstructionScript
  (|CallParentFunction))