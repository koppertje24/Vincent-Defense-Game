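; BP_Building_WindowFrame is a modular building piece for a window frame that handles removal of the window attached to it.
; It overrides RemoveAttachedObject to act on a valid WindowReference, forwarding the call to that window and then destroying it.
; When the Destruct flag is set, it first calls DestructMulticast with the window's destructible mesh and world transform.
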(event EventRemoveAttachedObject
  (params (Destruct :type Boolean))
  (bind _windowreference (Variables|References|GetWindowReference))
  ;[1 1 1] Overridden Events.
  (Utilities|IsValid _windowreference
    (:Is%20Valid
      (if Destruct
        (CallFunction|Destruct(Multicast) (.DestructibleMesh (Utilities|Struct|BreakSTR_BuildingObjectSettings (Variables|/Game/VVG/BP_Building_BuildingObject.BP_Building_BuildingObject_C|GetSettings _windowreference))) (Transformation|GetWorldTransform (Variables|/Game/VVG/BP_Building_BuildingObject.BP_Building_BuildingObject_C|GetMesh _windowreference))))
      (Default|RemoveAttachedObject _windowreference Destruct)
      (Actor|DestroyActor _windowreference))))

(fn ConstructionScript
  (|CallParentFunction))