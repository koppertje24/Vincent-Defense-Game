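; Behavior tree decorator that checks whether an AI character may chase its target.
; It casts the controlled pawn to BP_Character_Base and reads the TargetActor and GuardLocation blackboard values.
; The check passes when the target is valid and its distance from the guard location, not from the pawn, is less than the character's ChasingDistance, leashing the chase to the guarded spot.
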(fn PerformConditionCheckAI
  (params (OwnerController :type AI%20Controller%20Object%20Reference) (ControlledPawn :type Pawn%20Object%20Reference))
  (bind _targetactor (Variables|Blackboard|GetTargetActor))
  (bind _returnvalue (AI|BehaviorTree|GetBlackboardValueasActor _targetactor))
  ;[1 1 1] Check chasing conditions.
  (bind _asbp_character_base (Utilities|Casting|CastToBP_Character_Base ControlledPawn))
  (Utilities|IsValid _returnvalue
    (:Is%20Valid
      (return (> (Variables|/Game/VVG/BP_Character_Base.BP_Character_Base_C|GetChasingDistance _asbp_character_base) (Math|Vector|VectorLength (- (Transformation|GetActorLocation _returnvalue) (Class|BTFunctionLibrary|GetBlackboardValueasVector (Variables|Blackboard|GetGuardLocation)))))))))